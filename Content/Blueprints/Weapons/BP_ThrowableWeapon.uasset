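; Throwable weapon that launches from the character's hand and explodes after a countdown.
; Fire detaches the mesh, enables collision, sets projectile velocity from direction and charge, and starts a one-second looping timer that updates the countdown widget.
; At zero, a sphere overlap sends damage messages, spawning effect and sound per overlapped actor, then kills the weapon.
; Explosion radius comes from the throwable data table.
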(event `self.Fire`
  (params (Direction :type "Vector Structure") (Chage :type "Float (single-precision)"))
  (bind _projectilemovement (`self.ProjectileMovement`))
  ;[1 1 1] Throwable is fired
  (`PrimitiveComponent.SetCollisionEnabled` (`self.Weapon_SK_Mesh`) "QueryAndPhysics") ; Enables collison of the mesh
  (`self.K2_DetachFromActor` "KeepWorld" "KeepWorld" "KeepWorld") ; Detatch from the characters hand socket
  (`ActorComponent.SetActive` _projectilemovement true false) ; This activates the projectile component so that the object will fire in the correct direction
  (set `MovementComponent.Velocity` (* Direction (* Chage 200.0)) _projectilemovement)
  (set `self.countDownTimer` (`self.countDown`)) ; Set the timer to the timer value that has been set
  (`/Game/UI/Weapons/UI_ThrowableCountdown.Set Number` (`self.throwableCountdownUI`) (`self.countDownTimer`)) ; Set the inital starting number to the UI
  (`self.OnWeaponFired`)
  (bind _audiomanager (message `/Game/Interfaces/BPI_Audio.GetSoundManger` (`GameplayStatics.GetGameMode`)))
  (`/Game/Blueprints/Managers/BP_AudioManager.PlaySound` _audiomanager "Throw")
  ;[1 1 1] Timer of throwable
  (bind _returnvalue (`KismetSystemLibrary.K2_SetTimerDelegate` (delegate `SetUICountDown`) 1.0 true)) ; Timer counts each second
  (`SceneComponent.SetVisibility` (`self.Widget`) true false))

(event `StopTimer`
  ;[1 1 1] Timer of throwable
  (`KismetSystemLibrary.K2_ClearAndInvalidateTimerHandle` (stale `self.Fire` _returnvalue)) ; Stop the timer and clear it when it explodes
)

(event `SetUICountDown`
  ;[1 1 1] Timer of throwable
  (bind _result (`/Engine/EditorBlueprintResources/StandardMacros.DecrementFloat` (`self.countDownTimer`))
    (:`  `
      (if (> _result 0.0)
        (`/Game/UI/Weapons/UI_ThrowableCountdown.Set Number` (`self.throwableCountdownUI`) (`self.countDownTimer`)) ; Set the countdown number to the UI each second
        (else
          (`self.Explode`) ; When timer reaches 0 it explodes
          (`self.StopTimer`))))))

(event `self.KillWeapon`
  (bind _projectilemovement (`self.ProjectileMovement`))
  (`parent.KillWeapon`)
  (`ActorComponent.SetActive` _projectilemovement false false)
  (`MovementComponent.SetUpdatedComponent` _projectilemovement (`self.RootComponent`))
  (`self.StopTimer`)
  (`self.OnWeaponFinished`))

(event `self.InitWeapon`
  (params (`Weapon Name` :type Name) (`Weapon Manager` :type "/Game/Blueprints/Managers/BP_WeaponManager Object Reference"))
  ;[1 1 1] Init Weapon
  (`parent.InitWeapon` `Weapon Name` null)
  (`PrimitiveComponent.SetCollisionEnabled` (`self.Weapon_SK_Mesh`) "NoCollision") ; Set no collision so that the mesh collison will not affect character movement
  (bind _asui_throwable_countdown (cast `/Game/UI/Weapons/UI_ThrowableCountdown` (`WidgetComponent.GetWidget` (`self.Widget`)))) ; Cast is nessasery to get widdget compnent refrence on init
  (set `self.throwableCountdownUI` _asui_throwable_countdown) ; Variable is then saved so cast is only needed once
  (`SceneComponent.SetVisibility` (`self.Widget`) false false))

(fn `Explode`
  (bind _outactors (`KismetSystemLibrary.SphereOverlapActors` (`SceneComponent.K2_GetComponentLocation` (`self.Weapon_SK_Mesh`)) (`self.explosionRadus`) (`|MakeArray` "ObjectTypeQuery1" "ObjectTypeQuery2" "ObjectTypeQuery3" :!type "EObjectTypeQuery Enum")))
  (for _array_element _outactors
    (message `/Game/Interfaces/BPI_Damageable.TakeDamage` _array_element self)
    (`GameplayStatics.SpawnEmitterAtLocation` "/Game/Assets/Stl_explosion_vfx/Particles/red/P_r_Explosion_gr_lrg_01.P_r_Explosion_gr_lrg_01" (`SceneComponent.K2_GetComponentLocation` (`self.Weapon_SK_Mesh`)) (struct) (1.0 1.0 1.5))
    (bind _audiomanager (message `/Game/Interfaces/BPI_Audio.GetSoundManger` (`GameplayStatics.GetGameMode`)))
    (`/Game/Blueprints/Managers/BP_AudioManager.PlaySound` _audiomanager "GrenadeExpl"))
  (`self.KillWeapon`)
  (`self.OnWeaponFinished`))

(fn `GetFiredObject`
  (returns (Obj :type "Actor Object Reference"))
  (return self))

(fn `SetupVariables`
  (params (`Weapon Name` :type Name))
  (`parent.SetupVariables` `Weapon Name`)
  (bind _returnvalue (`|GetDataTableRow` "/Game/DataTables/Weapons/D_ThrowableTable.D_ThrowableTable" `Weapon Name`)
    (:`then`
      (set `self.explosionRadus` (`.ExplosionRadus_21_6E7FA5BD4567CC2AD28EEEBBD75CD9BA` (break `/Game/Structs/WeaponsandProjectiles/Struct_ThrowableWeapons` _returnvalue))))))

(fn `UserConstructionScript`
  (`parent.UserConstructionScript`))