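; Behavior tree service that, on activation, picks an enemy target for the AI pawn and writes it to the Target blackboard key.
; It gets enemy-team characters through the game mode, assuming the AI is always Blue and enemies Red.
; A DistanceScore macro buckets each enemy's distance into score bands stored in a map.
; The lowest score wins, so ties within a band go to the first key found rather than the nearest.
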(event `self.ReceiveActivationAI`
  (params (OwnerController :type "AIController Object Reference") (ControlledPawn :type "Pawn Object Reference"))
  (set `self.controlledPawn` ControlledPawn) ; Set Var for the controlled pawn
  ;[1 1 1] Gets all the characters from a team
  (bind _gamemode (message `/Game/Interfaces/BPI_GameModes.GetGameMode` (`GameplayStatics.GetGameMode`)))
  (bind _characters (`/Game/Blueprints/GameMode/GM_UnstableWorms.GetCharactersFromTeam` _gamemode "NewEnumerator0")) ; Get Red team as the AI will alway be on blue team and red team is the enemy
  (set `self.enemyCharacters` _characters)
  (`self.SetupCharacterScore`)
  (`self.GetClosest`)
  (bind _lowestscore (`self.FindCharacterWithLowestScore`))
  (`BTFunctionLibrary.SetBlackboardValueAsObject` (`self.target`) _lowestscore))

(fn `FindCharacterWithLowestScore`
  (returns (LowestScore :type "/Game/Blueprints/Characters/Player/BP_Character Object Reference"))
  (locals (tempLowestCharacterScore :type "/Game/Blueprints/Characters/Player/BP_Character Object Reference"))
  (bind _keys (`BlueprintMapLibrary.Map_Keys` (`self.charactersScore`)))
  ;[1 1 1] Set the first character to current lowest score to begin
  (set `local.tempLowestCharacterScore` (`|GetArrayItem` _keys))
  (for _array_element _keys
    ;[1 1 1] If the current character score is less than the lowest score then it becomes the new lowest character
    (if (< (`BlueprintMapLibrary.Map_Find` (`self.charactersScore`) _array_element) (`BlueprintMapLibrary.Map_Find` (`self.charactersScore`) (`local.tempLowestCharacterScore`)))
      (set `local.tempLowestCharacterScore` _array_element)))
  (return (`local.tempLowestCharacterScore`)))

(fn `GetClosest`
  (for _array_element (`self.enemyCharacters`)
    (`self.DistanceScore` (`KismetMathLibrary.Vector_Distance` (`Actor.K2_GetActorLocation` (`self.controlledPawn`)) (`Actor.K2_GetActorLocation` _array_element)) 1000.0 2500.0 5000.0 ; Finds a score based on the distance
      (:`<= MinDistance`
        (bind (_value _returnvalue) (`BlueprintMapLibrary.Map_Find` (`self.charactersScore`) _array_element))
        (if _returnvalue
          (`|VariableSetRef` _value)))
      (:`<= MidDistance`
        (if _returnvalue
          (`|VariableSetRef` _value 1)))
      (:`<= MaxDistance`
        (if _returnvalue
          (`|VariableSetRef` _value 2)))
      (:`> MaxDistance`
        (if _returnvalue
          (`|VariableSetRef` _value 3))))))

(fn `SetupCharacterScore`
  (for _array_element (`self.enemyCharacters`)
    (`BlueprintMapLibrary.Map_Add` (`self.charactersScore`) _array_element))
  (return))