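; Base class for pooled projectile bullets that fly from a weapon's fire point and explode on hit or overlap.
; Speed, explosion radius, mesh and impact sound come from a data table row, and Launch sets velocity from direction and charge with an attached fire emitter.
; Explode passes sphere-overlapped actors to the firing weapon for damage and spawns particles.
; KillProjectile hides and deactivates the actor for reuse.
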(event `/Game/Interfaces/Weapons/BPI_Bullets.InitBullet`
  (params (Name :type Name) (FirePoint :type "Vector Structure"))
  (`parent.InitBullet` Name FirePoint)
  (`SceneComponent.K2_SetWorldLocation` (`self.StaticMesh`) (`self.firePoint`) false false) ; Sets the starting pos to the weapons firepoint
  (`self.SetActive`))

(event `self.StaticMesh.OnComponentHit`
  (params (HitComponent :type "PrimitiveComponent Object Reference") (OtherActor :type "Actor Object Reference") (OtherComp :type "PrimitiveComponent Object Reference") (NormalImpulse :type "Vector Structure") (Hit :type "HitResult Structure (by ref)"))
  ;[1 1 1] When the static mesh hits another object it should trigger these events and then explode
  (`self.Explode` :!label _label))

(event `self.StaticMesh.OnComponentBeginOverlap`
  (params (OverlappedComponent :type "PrimitiveComponent Object Reference") (OtherActor :type "Actor Object Reference") (OtherComp :type "PrimitiveComponent Object Reference") (OtherBodyIndex :type Integer) (bFromSweep :type Boolean) (SweepResult :type "HitResult Structure (by ref)"))
  ;[1 1 1] When the static mesh hits another object it should trigger these events and then explode
  (goto _label))

(event `self.SetActive`
  ;[1 1 1] Sets the projectile active or disabled
  (`self.SetActorHiddenInGame` false)
  (`self.SetActorEnableCollision` true)
  (`self.SetActorTickEnabled` true))

(event `self.SetDisabled`
  ;[1 1 1] Sets the projectile active or disabled
  (`self.SetActorHiddenInGame` true)
  (`self.SetActorEnableCollision` false)
  (`self.SetActorTickEnabled` false))

(event `/Game/Interfaces/Weapons/BPI_Projectile.KillProjectile`
  ;[1 1 1] Disables the projectile so it can be reused
  (`self.SetDisabled`)
  (`SceneComponent.K2_SetWorldLocation` (`self.StaticMesh`) (0.0 0.0 0.0) false false)
  (`ActorComponent.SetActive` (`self.ProjectileMovement`) false false))

(fn `Explode`
  (bind _outactors (`KismetSystemLibrary.SphereOverlapActors` (`SceneComponent.K2_GetComponentLocation` (`self.StaticMesh`)) (`self.explosionRadius`) (`|MakeArray` "ObjectTypeQuery1" "ObjectTypeQuery2" "ObjectTypeQuery3" :!type "EObjectTypeQuery Enum"))) ; Spawn sphere explosion
  (`self.ProjectileExploded` _outactors) ; Call the exploded event so that the weapon that has fired the projectile can then deal its damage
  ;[1 1 1] Spawn explosion particles
  (`GameplayStatics.SpawnEmitterAtLocation` "/Game/Assets/Stl_explosion_vfx/Particles/red/P_r_Explosion_gr_lrg_01.P_r_Explosion_gr_lrg_01" (`SceneComponent.K2_GetComponentLocation` (`self.StaticMesh`)))
  (`ActorComponent.Deactivate` (`self.fireEmitter`)))

(fn `GetProjectile`
  (returns (Projectile :type "/Game/Blueprints/Weapons/Bullets/Projectile/BP_BaseProjectile Object Reference"))
  (return self))

(fn `Launch`
  (params (Direction :type "Vector Structure") (Charge :type "Float (double-precision)"))
  (returns (HitActors :type "Array of Actor Object Reference"))
  (bind _projectilemovement (`self.ProjectileMovement`))
  (`ActorComponent.SetActive` _projectilemovement true false) ; This activates the projectile component so that the object will fire in the correct direction
  (`MovementComponent.SetUpdatedComponent` (`self.ProjectileMovement`) (`self.RootComponent`))
  (set `MovementComponent.Velocity` (* Direction (* Charge (`self.projectileSpeed`))) _projectilemovement)
  (`/Engine/EditorBlueprintResources/StandardMacros.IsValid` (`self.fireEmitter`)
    (:`Is Valid`
      (`ActorComponent.Activate` (`self.fireEmitter`) true))
    (:`Is Not Valid`
      (bind _returnvalue (`GameplayStatics.SpawnEmitterAttached` "/Game/Assets/PolygonScifi/Particles/FX_Fire.FX_Fire" (`self.StaticMesh`) "None" (0.0 0.0 0.0) (struct) (1.0 1.0 1.0) "KeepRelativeOffset" false))
      (set `self.fireEmitter` _returnvalue)))
  (return))

(fn `SetupVariables`
  (params (Name :type Name) (FirePoint :type "Vector Structure"))
  (`parent.SetupVariables` Name FirePoint)
  (bind _returnvalue (`|GetDataTableRow` "/Game/DataTables/Weapons/D_ProjectileTable.D_ProjectileTable" Name)
    (:`then`
      (bind (_name _speed _explosionradus _mesh _impactsound) (break `/Game/Structs/WeaponsandProjectiles/Struct_ProjectileSettings` _returnvalue))
      (set `self.projectileSpeed` _speed)
      (set `self.explosionRadius` _explosionradus)
      (`StaticMeshComponent.SetStaticMesh` (`self.StaticMesh`) _mesh)
      (set `self.Impact Sound` _impactsound))))

(fn `UserConstructionScript`)