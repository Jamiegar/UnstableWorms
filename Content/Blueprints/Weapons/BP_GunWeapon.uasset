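; BP_GunWeapon is a gun weapon that plays a firing sound and launches either a projectile or ray trace, depending on bullet type.
; Setup extends the parent's, reading bullet name and sound from D_GunTable by weapon name.
; Firing looks up the bullet in the WeaponManager, then initialises and launches it from the muzzle socket through interface messages.
; Rays damage hit actors and finish immediately, while projectiles defer both until their exploded event.
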(event `/Game/Interfaces/Weapons/BPI_Weapons.Fire`
  (params (Direction :type "Vector Structure") (Chage :type "Float (single-precision)"))
  (bind _audiomanager (message `/Game/Interfaces/BPI_Audio.GetSoundManger` (`GameplayStatics.GetGameMode`)))
  (`/Game/Blueprints/Managers/BP_AudioManager.PlaySound` _audiomanager (`self.Firing Sound`))
  (switch `/Game/Enum/Weapons/FiringType` (`self.bulletType`)
    (:`NewEnumerator0`
      (`self.LaunchProjectileFromGun` Direction Chage))
    (:`NewEnumerator1`
      (`self.LaunchRayFromGun` Direction Chage))))

(event `OnProjectileExploded`
  (params (HitObjects :type "Array of Actor Object Reference"))
  (for _array_element HitObjects
    (message `/Game/Interfaces/BPI_Damageable.TakeDamage` _array_element self) ; Loops through all hit actors and calls the take damage func
  )
  (`self.OnWeaponFinished`) ; Weapon has finished firing
)

(fn `GetFiredObject`
  (returns (Obj :type "Actor Object Reference"))
  (return (`BlueprintMapLibrary.Map_Find` (`/Game/Blueprints/Managers/BP_WeaponManager.bullet` (`self.weaponManager`)) (`self.bulletName`))))

(fn `LaunchProjectileFromGun`
  (params (Direction :type "Vector Structure") (Charge :type "Float (double-precision)"))
  (bind _value (`BlueprintMapLibrary.Map_Find` (`/Game/Blueprints/Managers/BP_WeaponManager.bullet` (`self.weaponManager`)) (`self.bulletName`)))
  (message `/Game/Interfaces/Weapons/BPI_Bullets.InitBullet` _value (`self.weaponName`) (`SceneComponent.GetSocketLocation` (`self.Weapon_SK_Mesh`) "SK_Wep_FirePoint"))
  (`self.OnWeaponFired`)
  ;[1 1 1] Launches projectile
  (message `/Game/Interfaces/Weapons/BPI_Bullets.Launch` _value (`local.Direction`) (`local.Charge`))
  (bind _projectile (message `/Game/Interfaces/Weapons/BPI_Projectile.GetProjectile` _value)) ; Gets the base projectile
  ;[1 1 1] Bind to event that is called when the projectile explodes
  (add `/Game/Blueprints/Weapons/Bullets/Projectile/BP_BaseProjectile.ProjectileExploded` _projectile (`|CreateDelegate` :!event `OnProjectileExploded`)))

(fn `LaunchRayFromGun`
  (params (Direction :type "Vector Structure") (Charge :type "Float (double-precision)"))
  (bind _value (`BlueprintMapLibrary.Map_Find` (`/Game/Blueprints/Managers/BP_WeaponManager.bullet` (`self.weaponManager`)) (`self.bulletName`)))
  (message `/Game/Interfaces/Weapons/BPI_Bullets.InitBullet` _value (`self.weaponName`) (`SceneComponent.GetSocketLocation` (`self.Weapon_SK_Mesh`) "SK_Wep_FirePoint"))
  (`self.OnWeaponFired`)
  ;[1 1 1] Fires rays from weapon
  (bind _hitactors (message `/Game/Interfaces/Weapons/BPI_Bullets.Launch` _value (`local.Direction`) (`local.Charge`)))
  ;[1 1 1] Each actor hit has the take damage interface func called, if they implment func then they will become damaged
  (for _array_element _hitactors
    (message `/Game/Interfaces/BPI_Damageable.TakeDamage` _array_element self))
  (`self.OnWeaponFinished`) ; weapon finished firing
)

(fn `SetupVariables`
  (params (`Weapon Name` :type Name))
  (`parent.SetupVariables` `Weapon Name`)
  ;[1 1 1] Sets the bullet name for this weapon
  (bind _returnvalue (`|GetDataTableRow` "/Game/DataTables/Weapons/D_GunTable.D_GunTable" `Weapon Name`)
    (:`then`
      (bind (_bulletname _firingsound) (break `/Game/Structs/WeaponsandProjectiles/Struct_GunWeaponsSettings` _returnvalue))
      (set `self.bulletName` _bulletname)
      (set `self.Firing Sound` _firingsound))))

(fn `UserConstructionScript`)