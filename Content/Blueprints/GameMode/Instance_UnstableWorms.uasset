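; Game instance Blueprint for UnstableWorms that, as its name suggests, holds match settings.
; Events set the random map option, the AI option, and the character indices for the red and blue teams.
; GetGameSettings returns all stored values in a single call.
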(event `/Game/Interfaces/BPI_GameInstance.SetRandomMap`
  (params (RandomMap :type Boolean))
  (set `self.Random Map` RandomMap))

(event `/Game/Interfaces/BPI_GameInstance.SetUsingAI`
  (params (UsingAI :type Boolean))
  (set `self.Use AI` UsingAI))

(event `/Game/Interfaces/BPI_GameInstance.SetTeamCharacters`
  (params (RedTeamIndex :type Integer) (BlueTeamIndex :type Integer))
  (set `self.Red Team Index` RedTeamIndex)
  (set `self.Blue Team Index` BlueTeamIndex))

(fn `GetGameSettings`
  (returns (RandomMap :type Boolean) (UseAI :type Boolean) (RedTeamIndex :type Integer) (BlueTeamIndex :type Integer))
  (return (`self.Random Map`) (`self.Use AI`) (`self.Red Team Index`) (`self.Blue Team Index`)))