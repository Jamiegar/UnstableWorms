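; Weapon manager that pre-spawns and reuses one gun actor, one throwable actor and a set of bullet actors.
; Init spawns both weapons disabled, then SetupProjectiles adds one disabled instance of each bullet class to a class-keyed map.
; SpawnWeapon looks up a D_WeaponTable row, picks the pooled weapon by type, initializes it with the name and manager, activates it and returns it.
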(event `/Game/Interfaces/BPI_Initalize.Init`
  (bind _returnvalue (`|SpawnActorFromClass` "/Game/Blueprints/Weapons/BP_ThrowableWeapon.BP_ThrowableWeapon_C" (`KismetMathLibrary.MakeTransform` (0.0 0.0 0.0)) "Undefined" "OverrideRootScale" null null))
  (bind _output_get (set `self.throwableWeapon` _returnvalue))
  (message `/Game/Interfaces/BPI_Active.SetDisabled` _output_get)
  (bind _returnvalue_2 (`|SpawnActorFromClass` "/Game/Blueprints/Weapons/BP_GunWeapon.BP_GunWeapon_C" (`KismetMathLibrary.MakeTransform` (0.0 0.0 0.0)) "Undefined" "OverrideRootScale" null null))
  (bind _output_get_2 (set `self.gunWeapon` _returnvalue_2))
  (message `/Game/Interfaces/BPI_Active.SetDisabled` _output_get_2)
  (`self.SetupProjectiles`))

(fn `SetupProjectiles`
  (bind _returnvalue (`|SpawnActorFromClass` "/Game/Blueprints/Weapons/Bullets/LineTrace/BP_BulletRay.BP_BulletRay_C" (`KismetMathLibrary.MakeTransform` (0.0 0.0 0.0)) "Undefined" "OverrideRootScale" null null))
  (bind _output_get (set `self.rayBullet` _returnvalue))
  (`BlueprintMapLibrary.Map_Add` (`self.bullet`) "/Game/Blueprints/Weapons/Bullets/LineTrace/BP_BulletRay.BP_BulletRay_C" _output_get)
  (bind _returnvalue_2 (`|SpawnActorFromClass` "/Game/Blueprints/Weapons/Bullets/Projectile/BP_BulletProjectile.BP_BulletProjectile_C" (`KismetMathLibrary.MakeTransform` (0.0 0.0 0.0) (struct) (2.0 2.0 2.0)) "Undefined" "OverrideRootScale" null null))
  (bind _output_get_2 (set `self.scatterBullet` _returnvalue_2))
  (`BlueprintMapLibrary.Map_Add` (`self.bullet`) "/Game/Blueprints/Weapons/Bullets/Projectile/BP_BulletProjectile.BP_BulletProjectile_C" _output_get_2)
  (bind _returnvalue_3 (`|SpawnActorFromClass` "/Game/Blueprints/Weapons/Bullets/LineTrace/BP_ScatterRay.BP_ScatterRay_C" (`KismetMathLibrary.MakeTransform` (0.0 0.0 0.0) (struct) (2.0 2.0 2.0)) "Undefined" "OverrideRootScale" null null))
  (bind _output_get_3 (set `self.scatterPojectile` _returnvalue_3))
  (`BlueprintMapLibrary.Map_Add` (`self.bullet`) "/Game/Blueprints/Weapons/Bullets/LineTrace/BP_ScatterRay.BP_ScatterRay_C" _output_get_3)
  (bind _values (`BlueprintMapLibrary.Map_Values` (`self.bullet`)))
  (for _array_element _values
    (message `/Game/Interfaces/BPI_Active.SetDisabled` _array_element)))

(fn `SetUpWeapon`
  (params (Weapon :type "/Game/Blueprints/Weapons/BP_BaseWeapon Object Reference") (`Weapon Name` :type Name))
  (message `/Game/Interfaces/Weapons/BPI_Weapons.InitWeapon` Weapon `Weapon Name` self)
  (message `/Game/Interfaces/BPI_Active.SetActive` Weapon))

(fn `SpawnWeapon`
  (params (WeaponName :type Name))
  (returns (Weapon :type "/Game/Blueprints/Weapons/BP_BaseWeapon Object Reference"))
  (bind _returnvalue (`|GetDataTableRow` "/Game/DataTables/Weapons/D_WeaponTable.D_WeaponTable" WeaponName)
    (:`then`
      (bind (_weaponname _damage _weapontype) (break `/Game/Structs/WeaponsandProjectiles/Struct_WeaponSettings` _returnvalue))
      (switch `/Game/Enum/Weapons/WeaponType` _weapontype
        (:`NewEnumerator0`
          (`self.SetUpWeapon` (`self.gunWeapon`) _weaponname)
          (return (`self.gunWeapon`)))
        (:`NewEnumerator3`
          (`self.SetUpWeapon` (`self.throwableWeapon`) _weaponname)
          (return (`self.throwableWeapon`)))))))

(fn `UserConstructionScript`)