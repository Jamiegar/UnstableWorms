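; Behavior tree service that picks an AI character's weapon on activation and writes its name to the SelectedWeapon Blackboard key.
; It gets the controller's inventory and gathers WeaponsInInventory keys with values above zero.
; One candidate is picked at random, using an inclusive range up to the array length, which can overrun the last index.
; With no candidates, it falls back to the first key, commented as the always-owned weapon.
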(event `self.ReceiveActivationAI`
  (params (OwnerController :type "AIController Object Reference") (ControlledPawn :type "Pawn Object Reference"))
  ;[1 1 1] Get inventory
  (bind _inventory (message `/Game/Interfaces/BPI_Controllers.GetInventory` OwnerController))
  (set `self.Inventory` _inventory)
  (bind _potentialweapons (`self.GetPotentialWeapons`)) ; Gets Weapons in the inventory
  (if (<= (`KismetArrayLibrary.Array_Length` _potentialweapons) 0)
    ;[1 1 1] If <= 0 then index 0 is chosen as this is the weapon that the characters have always
    (`BTFunctionLibrary.SetBlackboardValueAsName` (`self.selectedWeapon`) (`self.GetWeaponNameAt` 0))
    (else
      ;[1 1 1] If false then a weapon from that list is chosen
      (bind _selectedweapon (`self.SelectWeaponAtRandom` _potentialweapons))
      (`BTFunctionLibrary.SetBlackboardValueAsName` (`self.selectedWeapon`) _selectedweapon))))

(fn `GetPotentialWeapons`
  (returns (potentialWeapons :type "Array of Name"))
  (locals (tempPotentialWeapons :type "Array of Name"))
  (bind _weaponsininventory (`/Game/Componenets/Com_Inventory.weaponsInInventory` (`self.Inventory`)))
  (bind _keys (`BlueprintMapLibrary.Map_Keys` _weaponsininventory))
  (for _array_element _keys
    (if (> (`BlueprintMapLibrary.Map_Find` _weaponsininventory _array_element) 0)
      (`KismetArrayLibrary.Array_Add` (`local.tempPotentialWeapons`) _array_element)))
  (return (`local.tempPotentialWeapons`)))

(fn `GetWeaponNameAt`
  (params (Index :type Integer))
  (returns (Weapon :type Name))
  (bind _keys (`BlueprintMapLibrary.Map_Keys` (`/Game/Componenets/Com_Inventory.weaponsInInventory` (`self.Inventory`))))
  (return (`|GetArrayItem` _keys Index)))

(fn `SelectWeaponAtRandom`
  (params (Weapons :type "Array of Name"))
  (returns (SelectedWeapon :type Name))
  (return (`|GetArrayItem` Weapons (`KismetMathLibrary.RandomIntegerInRange` 0 (`KismetArrayLibrary.Array_Length` Weapons)))))