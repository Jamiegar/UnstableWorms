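; Viewport camera actor for a turn-based game that moves between characters and follows projectiles.
; SetCameraPos attaches it to the new look-at actor, then chains timeline lerps out along negative Y and over to that actor, firing an event the turn component uses to start the next turn.
; A gate on Tick snaps it to the projectile until LerpToCurrentLookAtActor closes it, lerps back and reattaches.
; LerpToLocation moves it to any given point.
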(event `self.ReceiveTick`
  (params (DeltaSeconds :type "Float (single-precision)"))
  ;[1 1 1] Lerps camera to the curretn look at actor
  (`/Engine/EditorBlueprintResources/StandardMacros.Gate` true :!label _label ; Attaching the projectile opens the gate
    (:`Exit`
      (`self.K2_SetActorLocation` (`self.K2_GetActorLocation` (stale `AttachToProjectile` ParentActor))))))

(event `SetCameraPos`
  (params (LookAtActor :type "Actor Object Reference"))
  ;[1 1 1] Set Camera new look at pos and attach it to that actor
  (bind _output_get (set `self.lookAtActor` LookAtActor))
  (`self.K2_AttachToActor` _output_get "None" "KeepWorld" "SnapToTarget" "KeepWorld")
  (`self.LerpAwayFromCurrentCharacter`) ; After the character has been selected begin lerp transition
)

(event `AttachToProjectile`
  (params (ParentActor :type "Actor Object Reference"))
  ;[1 1 1] Lerps camera to the curretn look at actor
  (goto _label :!via `Open`))

(event `LerpToCurrentLookAtActor`
  ;[1 1 1] Lerps camera to the curretn look at actor
  (`|ExecutionSequence`
    (:`then_0`
      (goto _label :!via `Close`))
    (:`then_1`
      (bind (_direction _value) (`Timeline|Timeline_1` :!via `PlayFromStart`)
        (:`Update`
          (`SceneComponent.K2_SetWorldLocation` (`self.DefaultSceneRoot`) (`KismetMathLibrary.VLerp` (`self.K2_GetActorLocation`) (`self.K2_GetActorLocation` (`self.lookAtActor`)) _value) false false))
        (:`Finished`
          (`self.K2_AttachToActor` (`self.lookAtActor`) "None" "KeepWorld" "SnapToTarget" "KeepWorld"))))))

(event `LerpAwayFromCurrentCharacter`
  ;[1 1 1] Camrea inbetween turn lerps
  (set `self.zoomedOutVector` (- (`self.K2_GetActorLocation`) (`KismetMathLibrary.MakeVector` 0.0 (`self.lerpOutAmmount`)))) ; Set the pos of the target zoomed out location
  (bind (_direction _value) (`Timeline|LerpBetweenIn&Out` :!via `PlayFromStart`) ; Lerp between the curretn pos and the target zoomed out pos
    (:`Update`
      (`SceneComponent.K2_SetWorldLocation` (`self.DefaultSceneRoot`) (`KismetMathLibrary.VLerp` (`self.K2_GetActorLocation`) (`self.zoomedOutVector`) _value) false false))
    (:`Finished`
      (`self.LerpToNextCharacterPos`) ; On finished begin lerp to the next character
    )))

(event `LerpToNextCharacterPos`
  (bind _returnvalue_location (`KismetMathLibrary.BreakTransform` (`self.GetTransform` (`self.lookAtActor`))))
  ;[1 1 1] Camrea inbetween turn lerps
  (bind (_direction _value) (`Timeline|LerpBetweenPos` :!via `PlayFromStart`)
    (:`Update`
      (`SceneComponent.K2_SetWorldLocation` (`self.DefaultSceneRoot`) (`KismetMathLibrary.VLerp` (`self.K2_GetActorLocation`) _returnvalue_location _value) false false))
    (:`Finished`
      (`self.OnFinishedLerp`) ; This is called and then lissened to in the turn componet so that when the lerp is finsied the next turn can begin
    )))

(event `LerpToLocation`
  (params (Location :type "Vector Structure"))
  ;[1 1 1] Lerps camera to a location
  (bind (_direction _value) (`Timeline|Timeline_0` :!via `PlayFromStart`)
    (:`Update`
      (`SceneComponent.K2_SetWorldLocation` (`self.DefaultSceneRoot`) (`KismetMathLibrary.VLerp` (`self.K2_GetActorLocation`) Location _value) false false))))

(fn `UserConstructionScript`)