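; BP_UIManger is a UI manager Blueprint that creates and toggles the game's main HUD and pause menu.
; Its Init event creates UI_HUD and UI_PauseMenu, adds both to the viewport, initializes the HUD's messages and collapses the pause menu.
; DisplayPauseMenu swaps visibility between the two widgets, so both stay in the viewport and are shown or hidden rather than recreated.
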(event `/Game/Interfaces/BPI_Initalize.Init`
  ;[1 1 1] Create Main UI (all other UI should be on this and disabled and enabled when nessaserry)
  (bind _returnvalue (`|CreateWidget` "/Game/UI/UI_HUD.UI_HUD_C"))
  (bind _output_get (set `self.mainUI` _returnvalue))
  (`UserWidget.AddToViewport` _output_get 0)
  (message `/Game/Interfaces/BPI_Initalize.Init` _output_get)
  ;[1 1 1] Create pause menu
  (bind _returnvalue_2 (`|CreateWidget` "/Game/UI/Menus/Pause/UI_PauseMenu.UI_PauseMenu_C"))
  (bind _output_get_2 (set `self.pauseMenuUI` _returnvalue_2))
  (`UserWidget.AddToViewport` _output_get_2 0)
  (`Widget.SetVisibility` _output_get_2 "Collapsed"))

(fn `DisplayPauseMenu`
  (params (Display :type Boolean))
  (if Display
    (`Widget.SetVisibility` (`self.pauseMenuUI`) "Visible")
    (`Widget.SetVisibility` (`self.mainUI`) "Collapsed")
    (else
      (`Widget.SetVisibility` (`self.mainUI`) "Visible")
      (`Widget.SetVisibility` (`self.pauseMenuUI`) "Collapsed"))))

(fn `UserConstructionScript`)