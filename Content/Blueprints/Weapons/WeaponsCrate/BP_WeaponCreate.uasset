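; Weapon crate pickup that gives an overlapping character a random weapon.
; Init loads row names from the starting-weapons data table and picks one, skipping the first; the random range's upper bound is the array length, one past the last index.
; On overlap it runs Init if no weapon is set, then sends the weapon through BPI_Character, plays a pickup sound via the GameMode's sound manager and destroys itself.
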(event `/Game/Interfaces/BPI_Initalize.Init`
  (bind _outrownames (`DataTableFunctionLibrary.GetDataTableRowNames` "/Game/DataTables/Weapons/D_StartingWeapons.D_StartingWeapons"))
  (set `self.weaponNames` _outrownames)
  (`self.GetRandomWeapon`))

(event `self.Box.OnComponentBeginOverlap`
  (params (OverlappedComponent :type "PrimitiveComponent Object Reference") (OtherActor :type "Actor Object Reference") (OtherComp :type "PrimitiveComponent Object Reference") (OtherBodyIndex :type Integer) (bFromSweep :type Boolean) (SweepResult :type "HitResult Structure (by ref)"))
  ;[1 1 1] If the hit actor is a character then add the weapon in crate to rgw players inventory
  (if (not (!= (`self.weaponInCrate`) "None"))
    (`/Game/Interfaces/BPI_Initalize.Init`))
  (if (`KismetSystemLibrary.DoesImplementInterface` OtherActor "/Game/Interfaces/BPI_Character.BPI_Character_C")
    (message `/Game/Interfaces/BPI_Character.AddWeaponToPlayer` OtherActor (`self.weaponInCrate`))
    (bind _audiomanager (message `/Game/Interfaces/BPI_Audio.GetSoundManger` (`GameplayStatics.GetGameMode`)))
    (`/Game/Blueprints/Managers/BP_AudioManager.PlaySound` _audiomanager "CratePickup")
    (`self.K2_DestroyActor`)))

(fn `GetRandomWeapon`
  (bind _weaponnames (`self.weaponNames`))
  (set `self.weaponInCrate` (`|GetArrayItem` _weaponnames (`KismetMathLibrary.RandomIntegerInRange` 1 (`KismetArrayLibrary.Array_Length` _weaponnames)))))

(fn `UserConstructionScript`)