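; Base weapon actor for a turn-based game, with stub Fire and GetFiredObject for child weapons to override.
; InitWeapon loads mesh, stats and the character's reticle from a data table row and binds turn-end, fired and finished events.
; Handlers reach game systems through the GameMode to attach the camera to projectiles, stop the turn timer and return the camera.
; Weapons are detached, hidden or reset for reuse rather than destroyed.
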(event `self.InitWeapon`
  (params (`Weapon Name` :type Name) (`Weapon Manager` :type "/Game/Blueprints/Managers/BP_WeaponManager Object Reference"))
  (`self.SetupVariables` `Weapon Name`)
  (set `self.weaponManager` `Weapon Manager`)
  (bind _turn_system (message `/Game/Interfaces/BPI_GameModes.GetTurnComponent` (`GameplayStatics.GetGameMode`)))
  (add `/Game/Componenets/Com_TurnSystem.OnTurnEnd` _turn_system (`|CreateDelegate` :!event `OnTurnEnd`))
  (add `self.OnWeaponFired` (`|CreateDelegate` :!event `OnFired`))
  (add `self.OnWeaponFinished` (`|CreateDelegate` :!event `OnFinished`)))

(event `OnFinished`
  (bind _turn_system (message `/Game/Interfaces/BPI_GameModes.GetTurnComponent` (`GameplayStatics.GetGameMode`)))
  (`/Game/Componenets/Com_TurnSystem.StopCurrentTurnTimer` _turn_system)
  (bind _camera (message `/Game/Interfaces/BPI_GameModes.GetCamera` (`GameplayStatics.GetGameMode`)))
  (`/Game/Blueprints/Characters/BP_ViewportCamrea.LerpToCurrentLookAtActor` _camera))

(event `self.SetDisabled`
  ;[1 1 1] These are used when the weapons are not being used and should be hidden in game
  (`self.SetActorHiddenInGame` true)
  (`self.SetActorEnableCollision` false)
  (`self.SetActorTickEnabled` false))

(event `self.SetActive`
  ;[1 1 1] These are used when the weapons are not being used and should be hidden in game
  (`self.SetActorHiddenInGame` false)
  (`self.SetActorEnableCollision` true)
  (`self.SetActorTickEnabled` true))

(event `self.Fire`
  (params (Direction :type "Vector Structure") (Chage :type "Float (single-precision)"))
  (`KismetSystemLibrary.PrintString` "Base weapon")
  (`self.OnWeaponFired`)
  (`self.OnWeaponFinished`))

(event `self.KillWeapon`
  ;[1 1 1] If a weapon should hit the water it is killed so it can be reused
  (`self.SetDisabled`)
  (`SceneComponent.K2_SetWorldLocation` (`self.Weapon_SK_Mesh`) (0.0 0.0 0.0) false false)
  (`PrimitiveComponent.SetSimulatePhysics` (`self.Weapon_SK_Mesh`) false)
  (`self.OnWeaponFinished`))

(fn `GetFiredObject`
  (returns (Obj :type "Actor Object Reference"))
  (return null))

(fn `OnFired`
  (switch `/Game/Enum/Weapons/FiringType` (`self.bulletType`)
    (:`NewEnumerator0`
      (bind _obj (`self.GetFiredObject`))
      (bind _camera (message `/Game/Interfaces/BPI_GameModes.GetCamera` (`GameplayStatics.GetGameMode`)))
      (`/Game/Blueprints/Characters/BP_ViewportCamrea.AttachToProjectile` _camera _obj))))

(fn `OnTurnEnd`
  (`self.K2_DetachFromActor` "KeepWorld" "KeepWorld" "KeepWorld")
  (`self.SetDisabled`))

(fn `SetupReticule`
  (params (Reticle :type "Texture2D Object Reference"))
  (bind (_controller _character) (message `/Game/Interfaces/BPI_GameModes.GetCurrentController&Character` (`GameplayStatics.GetGameMode`)))
  (bind _reticle_ui (message `/Game/Interfaces/Weapons/BPI_ReticleUI.GetReticleUI` (`WidgetComponent.GetWidget` (`/Game/Blueprints/Characters/Player/BP_Character.Reticule` _character))))
  (`/Game/UI/Weapons/UI_Reticle.Init ReticleUI` _reticle_ui Reticle))

(fn `SetupVariables`
  (params (`Weapon Name` :type Name))
  ;[1 1 1] Sets all the weapon design data from the data table
  (bind _returnvalue (`|GetDataTableRow` "/Game/DataTables/Weapons/D_WeaponTable.D_WeaponTable" `Weapon Name`)
    (:`then`
      (bind (_weaponname _damage _weapontype _bullettype _weaponmesh _reticle _inventoryui_tex2d _explosionimpulse) (break `/Game/Structs/WeaponsandProjectiles/Struct_WeaponSettings` _returnvalue))
      (set `self.weaponName` _weaponname)
      (set `self.damage` _damage)
      (set `self.weaponType` _weapontype)
      (set `self.bulletType` _bullettype)
      (`SkinnedMeshComponent.SetSkinnedAssetAndUpdate` (`self.Weapon_SK_Mesh`) _weaponmesh true)
      (`self.SetupReticule` _reticle)
      (set `self.impulseExplosion` _explosionimpulse))))

(fn `UserConstructionScript`)