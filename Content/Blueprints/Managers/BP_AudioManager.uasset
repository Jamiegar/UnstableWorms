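; BP_AudioManager is an audio manager that plays non-spatial sound effects by name.
; On Init it copies every row of the D_SoundEffects data table into a name-to-sound map, then plays "BackgroundSFX".
; PlaySound looks a name up in that map and plays the result as a 2D, non-UI sound.
; GetSoundManger is an empty function with no returned value.
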(event `/Game/Interfaces/BPI_Initalize.Init`
  (`self.SetupSoundLibaray`)
  (`self.PlaySound` "BackgroundSFX"))

(fn `GetSoundManger`
  (returns (AudioManager :type "/Game/Blueprints/Managers/BP_AudioManager Object Reference"))
  (return null))

(fn `PlaySound`
  (params (SoundEffectName :type Name))
  (`GameplayStatics.PlaySound2D` (`BlueprintMapLibrary.Map_Find` (`self.soundLibray`) SoundEffectName) 1.0 1.0 0.0 null null false))

(fn `SetupSoundLibaray`
  (bind _outrownames (`DataTableFunctionLibrary.GetDataTableRowNames` "/Game/DataTables/D_SoundEffects.D_SoundEffects"))
  (for _array_element _outrownames
    (bind _returnvalue (`|GetDataTableRow` "/Game/DataTables/D_SoundEffects.D_SoundEffects" _array_element)
      (:`then`
        (bind (_soundname _sound) (break `/Game/Structs/Sounds/Struct_SoundEffects` _returnvalue))
        (`BlueprintMapLibrary.Map_Add` (`self.soundLibray`) _soundname _sound)))))

(fn `UserConstructionScript`)