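; BP_ScatterRay is a hitscan scatter-shot bullet that fires a burst of line traces in a random cone around the launch direction.
; Launch traces from FirePoint along the Visibility channel, with the elliptical cone sized by SpreadH and SpeedV and the length by Range.
; Each trace spawns a small explosion emitter at its impact point, without checking for a hit.
; Unique hit actors accumulate in Hits, which Launch returns; Charge is unused.
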(fn `Launch`
  (params (Direction :type "Vector Structure") (Charge :type "Float (double-precision)"))
  (returns (HitActors :type "Array of Actor Object Reference"))
  (locals (hits :type "Array of Actor Object Reference"))
  (bind _firepoint (`self.firePoint`))
  (for _ (range (+ (`self.scatterAmount`) 1))
    (bind _outhit (`KismetSystemLibrary.LineTraceSingle` _firepoint (+ _firepoint (* (`KismetMathLibrary.RandomUnitVectorInEllipticalConeInDegrees` Direction (* (`self.spreadH`) 2.0) (* (`self.speedV`) 2.0)) (`self.range`))) "TraceTypeQuery1"))
    (bind (_bblockinghit _binitialoverlap _time _distance _location _impactpoint _normal _impactnormal _physmat _hitactor) (`GameplayStatics.BreakHitResult` _outhit))
    (`GameplayStatics.SpawnEmitterAtLocation` "/Game/Assets/Stl_explosion_vfx/Particles/red/P_r_Explosion_gr_sm_06.P_r_Explosion_gr_sm_06" _impactpoint (struct) (0.3 0.3 0.3))
    (if (not (`KismetArrayLibrary.Array_Contains` (`local.hits`) _hitactor))
      (`KismetArrayLibrary.Array_Add` (`local.hits`) _hitactor)))
  (return (`local.hits`)))

(fn `UserConstructionScript`
  (`parent.UserConstructionScript`))