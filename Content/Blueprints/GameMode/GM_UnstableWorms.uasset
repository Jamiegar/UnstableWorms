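; Game mode for a turn-based, two-team Worms-style match, played by local players or against a Blue AI.
; A state switch chains pre-game and setup, spawning managers, camera, controllers and alternating-team characters from game-instance settings.
; Components handle turns, match timer and win checks; character deaths update rosters and can trigger the win screen.
; It also handles pausing and exposes getters for its managers.
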(event `self.ReceiveBeginPlay`
  (`self.SetupGameSettings`)
  (`self.Switch Game State` "NewEnumerator0"))

(event `Pre-Game`
  (`self.SetupAudioManger`)
  (`self.Setup Map`)
  (`self.Get Player Starts`)
  (`self.Switch Game State` "NewEnumerator3"))

(event `Game Setup`
  (`self.Setup Camera`)
  (`self.SetupControllers`)
  (`self.Setup Characters`)
  (`self.Setup UI Manager`)
  ;[1 1 1] Init weapon Manger (spawneds the types of weapons)
  (`self.Setup Weapon Manager`)
  ;[1 1 1] Initalizes turn system (starting team should always be red)
  (`/Game/Componenets/Com_TurnSystem.SetUpFirstTurn` (`self.Com_TurnSystem`) "NewEnumerator0" (`self.redCharacters`) (`self.blueCharacters`) (`self.controllers`))
  (`self.SetupGameTime`)
  (`self.Switch Game State` "NewEnumerator1"))

(event `In Game`)

(event `Post-Game`)

(event `Team Winning`
  (bind _winningteam (`self.FindWinningTeam`))
  (`self.SetupWinState` _winningteam))

(fn `CreatePlayerController`
  (params (Team :type "/Game/Enum/Teams Enum" :default "NewEnumerator0"))
  ;[1 1 1] Creates a new C_WormsController
  (bind _returnvalue (`GameplayStatics.CreatePlayer` -1))
  ;[1 1 1] Init controller and save reference
  (`KismetArrayLibrary.Array_Add` (`self.controllers`) _returnvalue)
  (message `/Game/Interfaces/BPI_Initalize.Init` _returnvalue)
  (`PlayerController.SetViewTargetWithBlend` _returnvalue (`self.camera`) 0.0 "VTBlend_Linear" 0.0 false)
  (message `/Game/Interfaces/BPI_Teams.Set Team` _returnvalue (`local.Team`)))

(fn `FindWinningTeam`
  (returns (WinningTeam :type "/Game/Enum/Teams Enum"))
  (bind _characters (`self.GetCharactersFromTeam` "NewEnumerator0"))
  (bind _characters_2 (`self.GetCharactersFromTeam` "NewEnumerator1"))
  (if (< (`KismetArrayLibrary.Array_Length` _characters_2) (`KismetArrayLibrary.Array_Length` _characters))
    (return "NewEnumerator1")
    (else
      (return "NewEnumerator0"))))

(fn `Get Player Starts`
  (bind _outactors (`GameplayStatics.GetAllActorsOfClass` "/Game/Blueprints/Characters/BP_SpawnPoint.BP_SpawnPoint_C"))
  (set `self.spawners` _outactors))

(fn `GetCamera`
  (returns (Camera :type "/Game/Blueprints/Characters/BP_ViewportCamrea Object Reference"))
  (return (`self.camera`)))

(fn `GetCharactersFromTeam`
  (params (Team :type "/Game/Enum/Teams Enum" :default "NewEnumerator0"))
  (returns (Characters :type "Array of /Game/Blueprints/Characters/Player/BP_Character Object Reference"))
  (switch `/Game/Enum/Teams` Team
    (:`NewEnumerator0`
      (return (`self.redCharacters`)))
    (:`NewEnumerator1`
      (return (`self.blueCharacters`)))))

(fn `GetCurrentController&Character`
  (returns (Controller :type "Controller Object Reference") (Character :type "/Game/Blueprints/Characters/Player/BP_Character Object Reference"))
  (bind _com_turnsystem (`self.Com_TurnSystem`))
  (return (`/Game/Componenets/Com_TurnSystem.currentController` _com_turnsystem) (`/Game/Componenets/Com_TurnSystem.currentCharacter` _com_turnsystem)))

(fn `GetGameMode`
  (returns (GameMode :type "/Game/Blueprints/GameMode/GM_UnstableWorms Object Reference"))
  (return self))

(fn `GetMapManger`
  (returns (`Map Manger` :type "/Game/Blueprints/Managers/BP_MapManager Object Reference"))
  (return (`self.mapManger`)))

(fn `GetSoundManger`
  (returns (AudioManager :type "/Game/Blueprints/Managers/BP_AudioManager Object Reference"))
  (return (`self.audioManager`)))

(fn `GetTurnComponent`
  (returns (`Turn System` :type "/Game/Componenets/Com_TurnSystem Object Reference"))
  (return (`self.Com_TurnSystem`)))

(fn `GetUIManger`
  (returns (`UI Manger` :type "/Game/Blueprints/Managers/BP_UIManger Object Reference"))
  (return (`self.uiManger`)))

(fn `GetWeaponsManager`
  (returns (`Weapons Manager` :type "/Game/Blueprints/Managers/BP_WeaponManager Object Reference"))
  (return (`self.weaponManager`)))

(fn `RemoveCharacter`
  (params (Character :type "/Game/Blueprints/Characters/Player/BP_Character Object Reference"))
  (bind _redcharacters (`self.redCharacters`))
  (bind _bluecharacters (`self.blueCharacters`))
  (bind _team (message `/Game/Interfaces/BPI_Teams.Get Team` Character))
  (switch `/Game/Enum/Teams` _team
    (:`NewEnumerator0`
      ;[1 1 1] Removes the dead character and updates the verables in the turn systerm
      (`KismetArrayLibrary.Array_RemoveItem` _redcharacters (`|GetArrayItem` _redcharacters (`KismetArrayLibrary.Array_Find` _redcharacters Character)))
      (set `/Game/Componenets/Com_TurnSystem.RedCharacters` (`self.redCharacters`) (`self.Com_TurnSystem`)))
    (:`NewEnumerator1`
      (`KismetArrayLibrary.Array_RemoveItem` _bluecharacters (`|GetArrayItem` _bluecharacters (`KismetArrayLibrary.Array_Find` _bluecharacters Character)))
      (set `/Game/Componenets/Com_TurnSystem.BlueCharacters` (`self.blueCharacters`) (`self.Com_TurnSystem`))))
  (`/Game/Componenets/Com_TurnSystem.StopCurrentTurnTimer` (`self.Com_TurnSystem`))
  (bind (_redteamdead _blueteamdead) (`/Game/Componenets/Com_ScoreStaes.CheckWin` (`self.Com_ScoreStaes`) (`self.redCharacters`) (`self.blueCharacters`)))
  (if _redteamdead
    (`self.SetupWinState` "NewEnumerator1")
    (elif _blueteamdead
      (`self.SetupWinState` "NewEnumerator0"))))

(fn `SetGameToPause`
  (params (`Display?` :type Boolean))
  (if `Display?`
    (`/Game/Blueprints/Managers/BP_UIManger.DisplayPauseMenu` (`self.uiManger`) true)
    (`GameplayStatics.SetGamePaused` true)
    (bind _controller (message `/Game/Interfaces/BPI_Controllers.GetController` (`|GetArrayItem` (`self.controllers`))))
    (set `PlayerController.bShowMouseCursor` true _controller)
    (`WidgetBlueprintLibrary.SetInputMode_GameAndUIEx` _controller null)
    (else
      (`/Game/Blueprints/Managers/BP_UIManger.DisplayPauseMenu` (`self.uiManger`) false)
      (`GameplayStatics.SetGamePaused` false)
      (bind _controller_2 (message `/Game/Interfaces/BPI_Controllers.GetController` (`|GetArrayItem` (`self.controllers`))))
      (set `PlayerController.bShowMouseCursor` false _controller_2)
      (`WidgetBlueprintLibrary.SetInputMode_GameAndUIEx` _controller_2 null))))

(fn `Setup Camera`
  (bind _returnvalue (`|SpawnActorFromClass` "/Game/Blueprints/Characters/BP_ViewportCamrea.BP_ViewportCamrea_C" (`KismetMathLibrary.MakeTransform` (4000.0 -4000.0 2300.0)) "Undefined" "OverrideRootScale" null null))
  (set `self.camera` _returnvalue))

(fn `Setup Characters`
  (for _array_element (`self.spawners`)
    ;[1 1 1] Spawn a character but changes the team each time
    (`/Engine/EditorBlueprintResources/StandardMacros.FlipFlop`
      (:`A`
        (bind _character (`self.Spawn Character` _array_element))
        (message `/Game/Interfaces/BPI_Initalize.Init` _character)
        ;[1 1 1] Bind characters to remove character func on the characters death
        (add `/Game/Blueprints/Characters/Player/BP_Character.OnCharcterDead` _character (`|CreateDelegate` :!event `RemoveCharacter`))
        ;[1 1 1] Set the character mesh that was selected in the game set up menu
        (`/Game/Blueprints/Characters/Player/BP_Character.SetMesh` _character (`|GetArrayItem` (`self.characterMeshArray`) (`self.redTeamCharacterIndex`))))
      (:`B`
        (bind _character_2 (`self.Spawn Character` _array_element "NewEnumerator1"))
        (message `/Game/Interfaces/BPI_Initalize.Init` _character_2)
        (add `/Game/Blueprints/Characters/Player/BP_Character.OnCharcterDead` _character_2 (`|CreateDelegate` :!event `RemoveCharacter`))
        (`/Game/Blueprints/Characters/Player/BP_Character.SetMesh` _character_2 (`|GetArrayItem` (`self.characterMeshArray`) (`self.blueTeamCharacterIndex`)))))))

(fn `Setup Map`
  (bind _returnvalue (`|SpawnActorFromClass` "/Game/Blueprints/Managers/BP_MapManager.BP_MapManager_C" (`KismetMathLibrary.MakeTransform` (0.0 0.0 0.0)) "Undefined" "OverrideRootScale" null null)) ; Spawn map manger
  (bind _output_get (set `self.mapManger` _returnvalue)) ; Save ref to manager
  (set `/Game/Blueprints/Managers/BP_MapManager.randomWorld` (`self.useRandomMap`) _output_get)
  (message `/Game/Interfaces/BPI_Initalize.Init` _output_get) ; Initalize the map manger which will spawn the map and find spawn points
)

(fn `Setup UI Manager`
  (bind _returnvalue (`|SpawnActorFromClass` "/Game/Blueprints/Managers/BP_UIManger.BP_UIManger_C" (`KismetMathLibrary.MakeTransform` (0.0 0.0 0.0)) "Undefined" "OverrideRootScale" null null))
  (bind _output_get (set `self.uiManger` _returnvalue))
  (message `/Game/Interfaces/BPI_Initalize.Init` _output_get))

(fn `Setup Weapon Manager`
  (bind _returnvalue (`|SpawnActorFromClass` "/Game/Blueprints/Managers/BP_WeaponManager.BP_WeaponManager_C" (`KismetMathLibrary.MakeTransform` (0.0 0.0 0.0)) "Undefined" "OverrideRootScale" null null))
  (bind _output_get (set `self.weaponManager` _returnvalue))
  (message `/Game/Interfaces/BPI_Initalize.Init` _output_get))

(fn `SetupAIControllers`
  (bind _returnvalue (`|SpawnActorFromClass` "/Game/Blueprints/Controllers/AI/AIC_WormsAIController.AIC_WormsAIController_C" (`KismetMathLibrary.MakeTransform` (0.0 0.0 0.0)) "Undefined" "OverrideRootScale" null null))
  (`KismetArrayLibrary.Array_Add` (`self.controllers`) _returnvalue)
  (message `/Game/Interfaces/BPI_Initalize.Init` _returnvalue)
  (message `/Game/Interfaces/BPI_Teams.Set Team` _returnvalue "NewEnumerator1"))

(fn `SetupAudioManger`
  (bind _returnvalue (`|SpawnActorFromClass` "/Game/Blueprints/Managers/BP_AudioManager.BP_AudioManager_C" (`KismetMathLibrary.MakeTransform` (0.0 0.0 0.0)) "Undefined" "OverrideRootScale" null null))
  (bind _output_get (set `self.audioManager` _returnvalue))
  (message `/Game/Interfaces/BPI_Initalize.Init` _output_get))

(fn `SetupControllers`
  ;[1 1 1] Removes the default controller
  (`GameplayStatics.RemovePlayer` (`GameplayStatics.GetPlayerController` 0))
  (if (`self.useAI`)
    (`self.CreatePlayerController` "NewEnumerator0")
    (`self.SetupAIControllers`)
    (else
      (for _ (range 1 (+ (`self.numberOfControllers`) 1))
        (`/Engine/EditorBlueprintResources/StandardMacros.FlipFlop`
          (:`A`
            (`self.CreatePlayerController` "NewEnumerator0"))
          (:`B`
            (`self.CreatePlayerController` "NewEnumerator1")))))))

(fn `SetupGameSettings`
  (bind (_randommap _useai _redteamindex _blueteamindex) (message `/Game/Interfaces/BPI_GameInstance.GetGameSettings` (`GameplayStatics.GetGameInstance`)))
  (set `self.useRandomMap` _randommap)
  (set `self.useAI` _useai)
  (set `self.redTeamCharacterIndex` _redteamindex)
  (set `self.blueTeamCharacterIndex` _blueteamindex))

(fn `SetupGameTime`
  (`/Game/Componenets/Com_GameTime.SetupGameTimer` (`self.Com_GameTime`) (`self.Com_TurnSystem`) (`self.uiManger`))
  (add `/Game/Componenets/Com_GameTime.OnGameTimerEnd` (`self.Com_GameTime`) (`|CreateDelegate` :!event `Team Winning`)))

(fn `SetupWinState`
  (params (WinningTeam :type "/Game/Enum/Teams Enum" :default "NewEnumerator0"))
  (bind _winui (`self.winUI`))
  (bind _winui_2 (`self.winUI`))
  (`/Game/Componenets/Com_TurnSystem.StopTurnSystem` (`self.Com_TurnSystem`))
  (bind _returnvalue (`|CreateWidget` "/Game/UI/Menus/WinScreen/UI_WinScreen.UI_WinScreen_C"))
  (bind _output_get (set `self.winUI` _returnvalue))
  (`UserWidget.AddToViewport` _output_get 0)
  (switch `/Game/Enum/Teams` WinningTeam
    (:`NewEnumerator0`
      (`/Game/UI/Menus/WinScreen/UI_WinScreen.SetWinningTeam` _winui_2 "NewEnumerator0")
      (message `/Game/Interfaces/BPI_Initalize.Init` _winui_2))
    (:`NewEnumerator1`
      (`/Game/UI/Menus/WinScreen/UI_WinScreen.SetWinningTeam` _winui "NewEnumerator1")
      (message `/Game/Interfaces/BPI_Initalize.Init` _winui)))
  (for _array_element (`self.controllers`)
    (bind _controller (message `/Game/Interfaces/BPI_Controllers.GetController` _array_element))
    (set `PlayerController.bShowMouseCursor` true _controller)
    (`WidgetBlueprintLibrary.SetInputMode_UIOnlyEx` _controller null)))

(fn `Spawn Character`
  (params (Spawner :type "/Game/Blueprints/Characters/BP_SpawnPoint Object Reference") (Team :type "/Game/Enum/Teams Enum" :default "NewEnumerator0"))
  (returns (Character :type "/Game/Blueprints/Characters/Player/BP_Character Object Reference"))
  ;[1 1 1] Spawns a character into the world on a spawn point
  (bind _returnvalue (`|SpawnActorFromClass` "/Game/Blueprints/Characters/Player/BP_Character.BP_Character_C" (`self.GetTransform` Spawner) "Undefined" "OverrideRootScale" null null))
  (message `/Game/Interfaces/BPI_Teams.Set Team` _returnvalue Team)
  (switch `/Game/Enum/Teams` Team
    (:`NewEnumerator0`
      ;[1 1 1] Adds character to array of its own team
      (`KismetArrayLibrary.Array_Add` (`self.redCharacters`) _returnvalue))
    (:`NewEnumerator1`
      (`KismetArrayLibrary.Array_Add` (`self.blueCharacters`) _returnvalue)))
  (return _returnvalue))

(fn `Switch Game State`
  (params (`Game State` :type "/Game/Enum/GameStates/GameStates Enum" :default "NewEnumerator0"))
  (switch `/Game/Enum/GameStates/GameStates` `Game State`
    (:`NewEnumerator0`
      ;[1 1 1] switches between the diffrent states (should be done it that order)
      (`self.Pre-Game`))
    (:`NewEnumerator3`
      (`self.Game Setup`))
    (:`NewEnumerator1`
      (`self.In Game`))
    (:`NewEnumerator2`
      (`self.Post-Game`))))

(fn `UserConstructionScript`)