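; Map manager that procedurally builds a destructible, side-on tile map for a turn-based game.
; Init loads data-table settings, optionally randomizes the seed, generates the map and binds to turn end.
; FastNoise values at or below a fill threshold become cube actors in a grid-keyed map, plus background and water.
; Open cells above tiles become spaced character spawn points, with leftovers feeding the weapon crate spawn component.
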(event `/Game/Interfaces/BPI_Initalize.Init`
  ;[1 1 1] Set Noise values from data table
  (bind _returnvalue (`|GetDataTableRow` "/Game/DataTables/Map/D_MapNoiseSettings.D_MapNoiseSettings" "DefaultNoise")
    (:`then`
      (if (`self.randomWorld`)
        (set `self.seed` (`KismetMathLibrary.RandomInteger` 5000))
        (else
          (bind (_seed _octaves _frequency _lacunarity) (break `/Game/Structs/Map/Struct_NoiseSettings` _returnvalue))
          (set `self.seed` _seed)))
      (set `self.octaves` _octaves)
      (set `self.frequency` _frequency)
      (set `self.lacunarity` _lacunarity)
      ;[1 1 1] Set map settings from data table
      (bind _returnvalue_2 (`|GetDataTableRow` "/Game/DataTables/Map/D_MapSettings.D_MapSettings" "DefaultMap")
        (:`then`
          (bind (_mapdimentions _fillvalue _fillactor) (break `/Game/Structs/Map/Struct_MapSettings` _returnvalue_2))
          (set `self.mapDimentions` _mapdimentions)
          (set `self.fillValue` _fillvalue)
          (set `self.cube` _fillactor)
          (`self.Genarate`)
          (bind _turn_system (message `/Game/Interfaces/BPI_GameModes.GetTurnComponent` (`GameplayStatics.GetGameMode`)))
          (add `/Game/Componenets/Com_TurnSystem.OnTurnEnd` _turn_system (`|CreateDelegate` (`self.Com_WeaponSpawn`) :!event `SpawnWeaponCrate`)))))))

(event `Genarate`
  (`self.FindCubeSize`)
  (`self.CreateNoiseMap`)
  (`self.FillMap`)
  (`self.SpawnBackground`)
  (`self.SpawnWater`)
  (`self.PlaceSpawnPointsintoWorld`)
  (`self.InitWeaponSpawns`))

(fn `CalcWorldPosition`
  (params (GridPosition :type "/Game/Structs/Map/Struct_GridDimentions Structure"))
  (returns (NewWorldPos :type "Vector Structure"))
  (locals (worldPos :type "Vector Structure"))
  (bind (_width _height) (break `/Game/Structs/Map/Struct_GridDimentions` GridPosition))
  (bind (_cubebounds_x _cubebounds_y _cubebounds_z) (`KismetMathLibrary.BreakVector` (`self.cubeBounds`)))
  (bind _output_get (set `local.worldPos` (`KismetMathLibrary.MakeVector` (* (* _width _cubebounds_x) 2.0) 0.0 (* (* _height _cubebounds_z) 2.0))))
  (return _output_get))

(fn `Clear`
  (for _array_element _
    (`self.K2_DestroyActor` _array_element)))

(fn `CreateNoiseMap`
  (locals (currentWidth :type Integer) (curretnHeight :type Integer))
  (bind (_mapdimentions_width _mapdimentions_height) (break `/Game/Structs/Map/Struct_GridDimentions` (`self.mapDimentions`)))
  (bind _returnvalue (`|GenericCreateObject` "/Script/FastNoiseGenerator.FastNoiseWrapper" self))
  (bind _output_get (set `self.noise` _returnvalue))
  (`FastNoiseWrapper.SetupFastNoise` _output_get "Simplex" (`self.seed`) (`self.frequency`) "Linear" "FBM" (`self.octaves`) (`self.lacunarity`) 0.5 0.45 "Euclidean" "CellValue")
  (for _index (range (+ _mapdimentions_width 1))
    (set `local.currentWidth` _index)
    (for _index_2 (range (+ _mapdimentions_height 1))
      (set `local.curretnHeight` _index_2)
      (`BlueprintMapLibrary.Map_Add` (`self.noiseMap`) (make `/Game/Structs/Map/Struct_GridDimentions` (`local.currentWidth`) (`local.curretnHeight`)) (`FastNoiseWrapper.GetNoise2D` (`self.noise`) (`KismetMathLibrary.Conv_IntToDouble` (`local.currentWidth`)) (`KismetMathLibrary.Conv_IntToDouble` (`local.curretnHeight`)))))))

(fn `DestroyNode`
  (params (`Grid Position` :type "/Game/Structs/Map/Struct_GridDimentions Structure"))
  (locals (tempNode :type "/Game/Blueprints/MapGenration/BP_GroundCube Object Reference"))
  (bind (_value _returnvalue) (`BlueprintMapLibrary.Map_Find` (`self.tilesOnGrid`) `Grid Position`))
  (set `local.tempNode` _value)
  (if _returnvalue
    (bind _returnvalue_2 (`BlueprintMapLibrary.Map_Remove` (`self.tilesOnGrid`) (`local.Grid Position`)))
    (if _returnvalue_2
      (`self.K2_DestroyActor` (`local.tempNode`)))))

(fn `FillMap`
  (locals (currentWidth :type Integer) (currentHeight :type Integer))
  (bind (_mapdimentions_width _mapdimentions_height) (break `/Game/Structs/Map/Struct_GridDimentions` (`self.mapDimentions`)))
  (bind (_value _returnvalue) (`BlueprintMapLibrary.Map_Find` (`self.noiseMap`) (make `/Game/Structs/Map/Struct_GridDimentions` (`local.currentWidth`) (`local.currentHeight`))))
  (bind _struct_griddimentions (make `/Game/Structs/Map/Struct_GridDimentions` (`local.currentWidth`) (`local.currentHeight`)))
  (for _index (range (+ _mapdimentions_width 1))
    (set `local.currentWidth` _index)
    (for _index_2 (range (+ _mapdimentions_height 1))
      (set `local.currentHeight` _index_2)
      (if _returnvalue
        (if (<= _value (`self.fillValue`))
          (bind _returnvalue_2 (`|SpawnActorFromClass` (`self.cube`) (`KismetMathLibrary.MakeTransform` (`self.CalcWorldPosition` (make `/Game/Structs/Map/Struct_GridDimentions` (`local.currentWidth`) (`local.currentHeight`)))) "Undefined" "OverrideRootScale" null null))
          (`BlueprintMapLibrary.Map_Add` (`self.tilesOnGrid`) _struct_griddimentions _returnvalue_2)
          (set `/Game/Blueprints/MapGenration/BP_GroundCube.GridPos` _struct_griddimentions _returnvalue_2)
          (`self.K2_AttachToActor` _returnvalue_2 self "None" "KeepRelative" "KeepRelative" "KeepRelative" true))))))

(fn `FindCubeSize`
  (bind _returnvalue (`|SpawnActorFromClass` (`self.cube`) (`self.GetTransform`) "Undefined" "OverrideRootScale" null null))
  (set `self.cubeBounds` (`.BoxExtent` (`self.GetActorBounds` _returnvalue false false)))
  (`self.K2_DestroyActor` _returnvalue))

(fn `FindSpawnPoints`
  (params (NumberOfSpawnPoints :type Integer))
  (returns (AllSpawnPoints :type "Array of /Game/Structs/Map/Struct_GridDimentions Structure"))
  (locals (potentialSpawnPoints :type "Array of /Game/Structs/Map/Struct_GridDimentions Structure") (SpawnPoints :type "Array of /Game/Structs/Map/Struct_GridDimentions Structure"))
  (bind _noisemap (`self.noiseMap`))
  (bind (_mapdimentions_width _mapdimentions_height) (break `/Game/Structs/Map/Struct_GridDimentions` (`self.mapDimentions`)))
  (bind _potentialspawnpoints (`local.potentialSpawnPoints`))
  (bind (_outitem _outindex) (`KismetArrayLibrary.Array_Random` _potentialspawnpoints))
  (bind _keys (`BlueprintMapLibrary.Map_Keys` _noisemap))
  (for _array_element _keys
    (bind (_value _returnvalue) (`BlueprintMapLibrary.Map_Find` _noisemap _array_element))
    (if _returnvalue
      ;[1 1 1] Find the positions on the grid that do not have tiles on them
      (if (> _value (`self.fillValue`))
        (bind (_width _height) (break `/Game/Structs/Map/Struct_GridDimentions` _array_element))
        (bind (_value_2 _returnvalue_2) (`BlueprintMapLibrary.Map_Find` (`self.tilesOnGrid`) (make `/Game/Structs/Map/Struct_GridDimentions` _width (- _height 1))))
        ;[1 1 1] if there is a node below and it is not == to null then it must be a solid block
        (if _returnvalue_2
          (`/Engine/EditorBlueprintResources/StandardMacros.IsValid` _value_2
            (:`Is Valid`
              ;[1 1 1] if it is already in the array then dont add it
              (if (not (`KismetArrayLibrary.Array_Contains` (`local.potentialSpawnPoints`) _array_element))
                (`KismetArrayLibrary.Array_Add` (`local.potentialSpawnPoints`) _array_element))))))
      (else
        (`KismetSystemLibrary.PrintString` "Could Not Find value in noise map" true true (struct :`R` 1.0 :`A` 1.0)))))
  (for _ (range (+ NumberOfSpawnPoints 1))
    (`KismetArrayLibrary.Array_Add` (`local.SpawnPoints`) _outitem) ; Add that random index to an array of the spawn points
    ;[1 1 1] Remove the tile from potential spawn points so it is not used again
    (`KismetArrayLibrary.Array_Remove` _potentialspawnpoints _outindex)
    ;[1 1 1] Removes all the neighbours from the potentail spawn points so that they cannot be used to spawn another character
    (for _array_element_2 (`self.SearchGridFromTile` _outitem)
      (bind (_width_2 _height_2) (break `/Game/Structs/Map/Struct_GridDimentions` _array_element_2))
      (if (not (or (> _width_2 _mapdimentions_width) (> _height_2 _mapdimentions_height) (< _width_2 0) (< _height_2 0)))
        (`KismetArrayLibrary.Array_RemoveItem` (`local.potentialSpawnPoints`) _array_element_2))))
  (set `self.potentialWeaponSpawns` (`local.potentialSpawnPoints`))
  (return (`local.SpawnPoints`)))

(fn `GetLastWeaponSpawnPoint`
  (returns (`Spawn Location` :type "Vector Structure"))
  (return (`/Game/Componenets/Com_WeaponSpawn.lastWeaponSpawnLocation` (`self.Com_WeaponSpawn`))))

(fn `GetMiddleTile`
  (returns (`Mid Tile` :type "/Game/Structs/Map/Struct_GridDimentions Structure"))
  (bind (_mapdimentions_width _mapdimentions_height) (break `/Game/Structs/Map/Struct_GridDimentions` (`self.mapDimentions`)))
  (return (make `/Game/Structs/Map/Struct_GridDimentions` (/ _mapdimentions_width 2) (/ _mapdimentions_height 2))))

(fn `InitWeaponSpawns`
  (locals (spawnLocations :type "Array of Vector Structure"))
  (for _array_element (`self.potentialWeaponSpawns`)
    (`KismetArrayLibrary.Array_Add` (`local.spawnLocations`) (`self.CalcWorldPosition` _array_element)))
  (`/Game/Componenets/Com_WeaponSpawn.InitWeaponSpawn` (`self.Com_WeaponSpawn`) (`local.spawnLocations`)))

(fn `PlaceSpawnPointsintoWorld`
  (bind _allspawnpoints (`self.FindSpawnPoints` 9))
  (for _array_element _allspawnpoints
    (`|SpawnActorFromClass` "/Game/Blueprints/Characters/BP_SpawnPoint.BP_SpawnPoint_C" (`KismetMathLibrary.MakeTransform` (`self.CalcWorldPosition` _array_element) (struct :`Yaw` -90.0)) "Undefined" "OverrideRootScale" null null)))

(fn `SearchGridFromTile`
  (params (StartingTileSearch :type "/Game/Structs/Map/Struct_GridDimentions Structure"))
  (returns (positions :type "Array of /Game/Structs/Map/Struct_GridDimentions Structure"))
  (locals (startingNode :type "/Game/Structs/Map/Struct_GridDimentions Structure") (nodes :type "Array of /Game/Structs/Map/Struct_GridDimentions Structure"))
  (bind (_startingnode_width _startingnode_height) (break `/Game/Structs/Map/Struct_GridDimentions` (`local.startingNode`)))
  (bind (_startingnode_width_2 _startingnode_height_2) (break `/Game/Structs/Map/Struct_GridDimentions` (`local.startingNode`)))
  (bind (_startingnode_width_3 _startingnode_height_3) (break `/Game/Structs/Map/Struct_GridDimentions` (`local.startingNode`)))
  (bind (_startingnode_width_4 _startingnode_height_4) (break `/Game/Structs/Map/Struct_GridDimentions` (`local.startingNode`)))
  (bind (_startingnode_width_5 _startingnode_height_5) (break `/Game/Structs/Map/Struct_GridDimentions` (`local.startingNode`)))
  (bind (_startingnode_width_6 _startingnode_height_6) (break `/Game/Structs/Map/Struct_GridDimentions` (`local.startingNode`)))
  (bind (_startingnode_width_7 _startingnode_height_7) (break `/Game/Structs/Map/Struct_GridDimentions` (`local.startingNode`)))
  (bind (_startingnode_width_8 _startingnode_height_8) (break `/Game/Structs/Map/Struct_GridDimentions` (`local.startingNode`)))
  (set `local.startingNode` StartingTileSearch)
  (bind _output_get (set `local.nodes` (`|MakeArray` (make `/Game/Structs/Map/Struct_GridDimentions` _startingnode_width_8 (+ _startingnode_height_8 1)) (make `/Game/Structs/Map/Struct_GridDimentions` _startingnode_width_7 (- _startingnode_height_7 1)) (make `/Game/Structs/Map/Struct_GridDimentions` (- _startingnode_width_4 1) _startingnode_height_4) (make `/Game/Structs/Map/Struct_GridDimentions` (+ _startingnode_width_5 1) _startingnode_height_5) (make `/Game/Structs/Map/Struct_GridDimentions` (+ _startingnode_width 1) (+ _startingnode_height 1)) (make `/Game/Structs/Map/Struct_GridDimentions` (+ _startingnode_width_3 1) (- _startingnode_height_3 1)) (make `/Game/Structs/Map/Struct_GridDimentions` (- _startingnode_width_6 1) (- _startingnode_height_6 1)) (make `/Game/Structs/Map/Struct_GridDimentions` (- _startingnode_width_2 1) (+ _startingnode_height_2 1)))))
  (return _output_get))

(fn `SpawnBackground`
  (bind _mid_tile (`self.GetMiddleTile`))
  (`|SpawnActorFromClass` "/Game/Blueprints/MapGenration/BP_Background.BP_Background_C" (`KismetMathLibrary.MakeTransform` (- (`self.CalcWorldPosition` _mid_tile) (0.0 -5000.0 0.0))) "Undefined" "OverrideRootScale" null null))

(fn `SpawnWater`
  (bind _mid_tile (`self.GetMiddleTile`))
  (`|SpawnActorFromClass` "/Game/Blueprints/MapGenration/BP_GroundWater.BP_GroundWater_C" (`KismetMathLibrary.MakeTransform` (`self.CalcWorldPosition` (make `/Game/Structs/Map/Struct_GridDimentions` (break `/Game/Structs/Map/Struct_GridDimentions` _mid_tile)))) "Undefined" "OverrideRootScale" null null))

(fn `SpawnWeapon`
  (`/Game/Componenets/Com_WeaponSpawn.SpawnWeaponCrate` (`self.Com_WeaponSpawn`)))

(fn `UserConstructionScript`)