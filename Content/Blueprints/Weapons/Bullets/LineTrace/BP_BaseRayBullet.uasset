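; BP_BaseRayBullet is a hitscan bullet Blueprint in the weapons folder that resolves a shot instantly with a line trace.
; Launch traces the Visibility channel from FirePoint along Direction for Range, then spawns a half-scale explosion emitter at the impact point.
; It appends the hit actor to Hits and returns that array, without checking whether the trace hit or using the Charge input.
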(fn `Launch`
  (params (Direction :type "Vector Structure") (Charge :type "Float (double-precision)"))
  (returns (HitActors :type "Array of Actor Object Reference"))
  (locals (hits :type "Array of Actor Object Reference"))
  (bind _firepoint (`self.firePoint`))
  (bind _outhit (`KismetSystemLibrary.LineTraceSingle` _firepoint (+ _firepoint (* Direction (`self.range`))) "TraceTypeQuery1"))
  (bind (_bblockinghit _binitialoverlap _time _distance _location _impactpoint _normal _impactnormal _physmat _hitactor) (`GameplayStatics.BreakHitResult` _outhit))
  (`KismetArrayLibrary.Array_Add` (`local.hits`) _hitactor)
  (`GameplayStatics.SpawnEmitterAtLocation` "/Game/Assets/Stl_explosion_vfx/Particles/red/P_r_Explosion_gr_sm_05.P_r_Explosion_gr_sm_05" _impactpoint (struct) (0.5 0.5 0.5))
  (return (`local.hits`)))

(fn `UserConstructionScript`
  (`parent.UserConstructionScript`))